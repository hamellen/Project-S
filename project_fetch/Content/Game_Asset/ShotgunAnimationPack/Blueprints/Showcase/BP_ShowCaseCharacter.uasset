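; Showcase character for a shotgun animation pack that repeatedly plays a chosen montage, single animation or full reload sequence.
; Reloads chain chamber, init, loop and finish montages based on ammo counts, then reset and repeat; shooting montages are followed by chambering.
; Montage notifies drive HandleNotifies, which plays matching weapon montages, moves the shell between sockets, updates ammo and spawns ejected casings.
; The construction script caches ammo defaults and optionally switches to first-person arms.
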(event `self.ReceiveBeginPlay`
  (bind _mesh (`self.Mesh`))
  (bind _montagetoplay (`self.MontageToPlay`))
  ;[1 1 1] Play a montage on begin play
  (if (`self.PlayReload?`)
    (`self.PlayReloadAnim`)
    (else
      (`/Engine/EditorBlueprintResources/StandardMacros.IsValid` _montagetoplay
        (:`Is Valid`
          (bind _notifyname (`|PlayMontage` (`self.Mesh`) _montagetoplay :!label _label)
            (:`OnBlendOut`
              (if (`self.IsShootingMontage?`)
                (`KismetSystemLibrary.Delay` 0.2)
                (bind _notifyname_2 (`|PlayMontage` (`self.Mesh`) "/Game/Game_Asset/ShotgunAnimationPack/Animations/Character/Montages/Montage_Shotgun_Chamber.Montage_Shotgun_Chamber")
                  (:`OnCompleted`
                    (`KismetSystemLibrary.Delay` 0.2 :!label _label_2)
                    (`self.ResetAmmo`)
                    (goto _label))
                  (:`OnNotifyBegin`
                    (`self.HandleNotifies` _notifyname_2)))
                (else
                  (goto _label_2))))
            (:`OnNotifyBegin`
              (`self.HandleNotifies` _notifyname))))
        (:`Is Not Valid`
          (`/Engine/EditorBlueprintResources/StandardMacros.IsValid` (`self.SingleAnimation`)
            (:`Is Valid`
              (`SkeletalMeshComponent.SetAnimationMode` _mesh "AnimationSingleNode" true)
              (`SkeletalMeshComponent.PlayAnimation` _mesh (`self.SingleAnimation`) true))))))))

(event `PlayMontageOnWeapon`
  (params (Montage :type "AnimMontage Object Reference"))
  ;[1 1 1] Play a montage on the weapon
  (bind _notifyname (`|PlayMontage` (`self.Shotgun`) Montage)
    (:`OnNotifyBegin`
      (switch `name` _notifyname
        (:`ShellLoaded`
          (`SceneComponent.K2_AttachToComponent` (`self.ShellToLoad`) (`self.Shotgun`) "ShellInMagSocket" "SnapToTarget" "SnapToTarget" "KeepRelative" true))))))

(event `PlayReloadAnim`
  ;[1 1 1] Handle reloading
  (`KismetSystemLibrary.Delay` 0.5)
  (if (== (`self.CurrentAmmo`) 0)
    (bind _notifyname (`|PlayMontage` (`self.GetTheMesh`) "/Game/Game_Asset/ShotgunAnimationPack/Animations/Character/Montages/Montage_Shotgun_ReloadInitChamber.Montage_Shotgun_ReloadInitChamber")
      (:`OnCompleted`
        (if (`self.CanReload?`)
          (bind _notifyname_2 (`|PlayMontage` (`self.GetTheMesh`) "/Game/Game_Asset/ShotgunAnimationPack/Animations/Character/Montages/Montage_Shotgun_ReloadInit.Montage_Shotgun_ReloadInit" :!label _label_3)
            (:`OnBlendOut`
              (if (`self.CanReload?`)
                (if (or (== (`self.InventoryAmmo`) 1) (== (- (`self.MaxAmmo`) (`self.CurrentAmmo`)) 1))
                  (bind _notifyname_3 (`|PlayMontage` (`self.GetTheMesh`) "/Game/Game_Asset/ShotgunAnimationPack/Animations/Character/Montages/Montage_Shotgun_ReloadFinish.Montage_Shotgun_ReloadFinish" :!label _label_4)
                    (:`OnCompleted`
                      (`self.ResetAmmo`))
                    (:`OnNotifyBegin`
                      (`self.HandleNotifies` _notifyname_3)))
                  (else
                    (bind _notifyname_4 (`|PlayMontage` (`self.GetTheMesh`) "/Game/Game_Asset/ShotgunAnimationPack/Animations/Character/Montages/Montage_Shotgun_ReloadLoop.Montage_Shotgun_ReloadLoop" :!label _label_5)
                      (:`OnBlendOut`
                        (if (and (`self.CanReload?`) (or (== (- (`self.MaxAmmo`) (`self.CurrentAmmo`)) 1) (== (`self.InventoryAmmo`) 1)))
                          (goto _label_4)
                          (elif (`self.CanReload?`)
                            (goto _label_5)
                            (else
                              (`self.ResetAmmo`)))))
                      (:`OnNotifyBegin`
                        (`self.HandleNotifies` _notifyname_4)))))
                (else
                  (`self.ResetAmmo`))))
            (:`OnNotifyBegin`
              (`self.HandleNotifies` _notifyname_2)))
          (else
            (`self.ResetAmmo`))))
      (:`OnNotifyBegin`
        (`self.HandleNotifies` _notifyname)))
    (else
      (goto _label_3))))

(fn `CanReload?`
  (returns (ReturnValue :type Boolean))
  (return (and (> (`self.InventoryAmmo`) 0) (< (`self.CurrentAmmo`) (`self.MaxAmmo`)))))

(fn `GetTheMesh`
  (returns (Mesh :type "SkeletalMeshComponent Object Reference"))
  (return (`self.Mesh`)))

(fn `HandleNotifies`
  (params (NotifyName :type Name))
  ;[1 1 1] Based on montage notify we determine what animation the shotgun should play and also play any necessary effects
  (switch `name` NotifyName
    (:`ShellIn`
      (`SceneComponent.K2_AttachToComponent` (`self.ShellToLoad`) (`self.Shotgun`) "ShellToLoadSocket" "SnapToTarget" "SnapToTarget" "KeepRelative" true)
      (`self.PlayMontageOnWeapon` "/Game/Game_Asset/ShotgunAnimationPack/Animations/Shotgun/Montages/Montage_Weapon_LoadShell.Montage_Weapon_LoadShell")
      (`/Engine/EditorBlueprintResources/StandardMacros.IncrementInt` (`self.CurrentAmmo`) :!label _label
        (:`  `
          (`/Engine/EditorBlueprintResources/StandardMacros.DecrementInt` (`self.InventoryAmmo`)))))
    (:`ShellChamberPrep`
      (`|ExecutionSequence`
        (:`then_0`
          (goto _label))
        (:`then_1`
          (`SceneComponent.K2_AttachToComponent` (`self.ShellToLoad`) (`self.GetTheMesh`) "ShellToChamber" "SnapToTarget" "SnapToTarget" "KeepRelative" true))))
    (:`ChamberShellIn`
      (`SceneComponent.K2_AttachToComponent` (`self.ShellToLoad`) (`self.Shotgun`) "ShellInChamberSocket" "SnapToTarget" "SnapToTarget" "KeepRelative" true))
    (:`ShellPrep`
      (`SceneComponent.K2_AttachToComponent` (`self.ShellToLoad`) (`self.GetTheMesh`) "ShellIn" "SnapToTarget" "SnapToTarget" "KeepRelative" true))
    (:`Pump_Chamber`
      (`self.PlayMontageOnWeapon` "/Game/Game_Asset/ShotgunAnimationPack/Animations/Shotgun/Montages/Montage_Weapon_Pump.Montage_Weapon_Pump"))
    (:`Pump_Lock`
      (`self.PlayMontageOnWeapon` "/Game/Game_Asset/ShotgunAnimationPack/Animations/Shotgun/Montages/Montage_Weapon_PumpLock.Montage_Weapon_PumpLock"))
    (:`Pump_Release`
      (`self.PlayMontageOnWeapon` "/Game/Game_Asset/ShotgunAnimationPack/Animations/Shotgun/Montages/Montage_Weapon_PumpRelease.Montage_Weapon_PumpRelease"))
    (:`EjectShell`
      ;;[1 1 1] Eject shell
      (bind _returnvalue (`|SpawnActorFromClass` "/Game/Game_Asset/ShotgunAnimationPack/Blueprints/Shotgun/BP_EjectedShell.BP_EjectedShell_C" (`KismetMathLibrary.MakeTransform` (.location (`SceneComponent.GetSocketTransform` (`self.Shotgun`) "EjectedShell" "RTS_World")) (.rotation (`SceneComponent.GetSocketTransform` (`self.Shotgun`) "EjectedShell" "RTS_World"))) "AdjustIfPossibleButAlwaysSpawn" "MultiplyWithRoot" null null))
      (`PrimitiveComponent.AddImpulse` (`StaticMeshActor.StaticMeshComponent` _returnvalue) (+ (* (`self.GetActorRightVector`) 20.0) (* (`self.GetActorUpVector`) 5.0)) "None" false))
    (:`ChamberCheck`
      (`|ExecutionSequence`
        (:`then_0`
          (`SceneComponent.K2_AttachToComponent` (`self.ShellToLoad`) (`self.Shotgun`) (select `bool` (== (`self.CurrentAmmo`) 0) :`false` "ShellInChamberSocket" :`true` "ShellHidden" :!type "Name") "SnapToTarget" "SnapToTarget" "KeepRelative" true :!label _label_2))
        (:`then_1`
          (`self.PlayMontageOnWeapon` "/Game/Game_Asset/ShotgunAnimationPack/Animations/Shotgun/Montages/Montage_Weapon_ChamberCheck.Montage_Weapon_ChamberCheck"))))
    (:`MagCheck`
      (`|ExecutionSequence`
        (:`then_0`
          (`SceneComponent.K2_AttachToComponent` (`self.ShellToLoad`) (`self.Shotgun`) (select `bool` (> (`self.CurrentAmmo`) 1) :`false` "ShellHidden" :`true` "ShellInMagSocket" :!type "Name") "SnapToTarget" "SnapToTarget" "KeepRelative" true))
        (:`then_1`
          (`self.PlayMontageOnWeapon` "/Game/Game_Asset/ShotgunAnimationPack/Animations/Shotgun/Montages/Montage_Weapon_MagCheck.Montage_Weapon_MagCheck"))))
    (:`InspectPump`
      (`|ExecutionSequence`
        (:`then_0`
          (goto _label_2))
        (:`then_1`
          (`self.PlayMontageOnWeapon` "/Game/Game_Asset/ShotgunAnimationPack/Animations/Shotgun/Montages/Montage_Weapon_Inspect.Montage_Weapon_Inspect"))))))

(fn `ResetAmmo`
  (`SceneComponent.K2_AttachToComponent` (`self.ShellToLoad`) (`self.Shotgun`) "ShellHidden" "SnapToTarget" "SnapToTarget" "KeepRelative" true)
  (set `self.InventoryAmmo` (`self.InventoryAmmo_Default`))
  (set `self.CurrentAmmo` (`self.CurrentAmmo_Default`))
  (if (`self.PlayReload?`)
    (`self.PlayReloadAnim`)))

(fn `UserConstructionScript`
  (set `self.CurrentAmmo_Default` (`self.CurrentAmmo`))
  (set `self.InventoryAmmo_Default` (`self.InventoryAmmo`))
  (if (`self.IsFP`)
    (`SkinnedMeshComponent.SetSkinnedAssetAndUpdate` (`self.Mesh`) "/Game/Game_Asset/ShotgunAnimationPack/Demo/Mannequin/Character/Mesh/SK_MannequinArms.SK_MannequinArms" true)))